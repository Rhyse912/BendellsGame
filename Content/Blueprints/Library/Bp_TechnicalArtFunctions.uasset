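; Technical art function library with a helper that recolors a material shared across a component hierarchy.
; ModifyBaseMaterialColor creates a dynamic material instance on a base mesh slot and sets the named color parameter on it.
; It then walks the root's child components, optionally all descendants, and assigns that single shared instance to static meshes whose same slot holds a material matching the original's name.
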(fn ModifyBaseMaterialColor
  (params (BaseStatic :type Static%20Mesh%20Component%20Object%20Reference) (MaterialIndex :type Integer) (MaterialColorName :type Name) (PaintColor :type Linear%20Color%20Structure) (Root :type Scene%20Component%20Object%20Reference) (IncludeAllDescendents :type Boolean))
  (LocalVariables|Setoriginal_mat_name (Utilities|GetObjectName (Rendering|Material|GetMaterial BaseStatic MaterialIndex)))
  (bind _returnvalue (Rendering|Material|CreateDynamicMaterialInstance BaseStatic MaterialIndex 0 :!class /Script/Engine.PrimitiveComponent))
  (Rendering|Material|SetVectorParameterValue _returnvalue MaterialColorName PaintColor :!class /Script/Engine.MaterialInstanceDynamic)
  (for _array_element (Components|GetChildrenComponents Root IncludeAllDescendents)
    (bind _asstatic_mesh_component (Utilities|Casting|CastToStaticMeshComponent _array_element))
    (if (Utilities|Enum|Equal(Enum) (Utilities|GetObjectName (Rendering|Material|GetMaterial _asstatic_mesh_component MaterialIndex)) (LocalVariables|Getoriginal_mat_name))
      (Rendering|Material|SetMaterial _asstatic_mesh_component MaterialIndex _returnvalue))))