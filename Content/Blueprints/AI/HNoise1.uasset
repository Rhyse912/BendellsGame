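; AI character HNoise1 that wanders to a random navigable point, heads to its Destination, then destroys itself on arrival.
; BeginPlay waits briefly, validates Destination, then chains AIMoveTo calls via a point around CircleCenter.
; Tick restarts movement through a nearby random point whenever the moving pawn stalls.
; BrainTick's line-of-sight player search is never called here, and the shooting, aiming and range functions are mostly stubs.
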(event EventBeginPlay
  ;[1 1 1] Begin play events
  ;;[1 1 1] Delay for 1 second and then proceed to destination
  (Utilities|FlowControl|Delay 1.0)
  (if (AI|IsValidAILocation (Variables|Default|GetDestination))
    (Variables|Default|SetIsMoving true)
    (Variables|/Script/Engine.CharacterMovementComponent|SetMaxWalkSpeed (Variables|Character|GetCharacterMovement) (Variables|Default|GetMovementSpeed))
    (AI|AIMoveTo self (.RandomLocation (Class|NavigationSystem|GetRandomPointinNavigableRadius (Variables|Default|GetCircleCenter) 1e+03)) 0 25.0 false
      (:OnSuccess
        _)
      (:OnFail
        _))
    (AI|AIMoveTo self (Variables|Default|GetDestination) 0 2.5e+02 false
      (:OnSuccess
        (Actor|DestroyActor)))))

(event EventTick
  (params (DeltaSeconds :type Float%20%28single-precision%29))
  (bind _self self)
  (bind _capsulecomponent (Variables|Collision|GetCapsuleComponent))
  (bind _returnvalue (Transformation|GetWorldLocation _capsulecomponent))
  (bind _randomlocation (Class|NavigationSystem|GetRandomPointinNavigableRadius _returnvalue 3e+02))
  ;[1 1 1] Tick events
  (if (and (<= (Math|Vector|VectorLength (Variables|/Script/Engine.MovementComponent|GetVelocity (Variables|Character|GetCharacterMovement))) 0.0) (Variables|Default|GetIsMoving))
    (Components|Movement|StopMovementImmediately (Variables|Character|GetCharacterMovement))
    (AI|AIMoveTo _self _randomlocation 0 25.0 false
      (:OnSuccess
        _)
      (:OnFail
        (AI|AIMoveTo self _randomlocation 0 25.0 false
          (:OnSuccess
            _))))
    (AI|AIMoveTo _self (Variables|Default|GetDestination) 0 2.5e+02 false
      (:OnSuccess
        (Actor|DestroyActor)))))

(event EventAssignDestination
  ;[1 1 1] Begin play events
  ;;[1 1 1] Accept destination
  (Variables|Default|SetDestination "0, 0, 0"))

(fn ConstructionScript)

(fn BrainTick
  (switch Utilities|FlowControl|Switch|Switchon (Variables|Default|GetAIState)
    (:NewEnumerator0
      (CallFunction|VisualSearch))))

(fn ShootatTarget)

(fn VisualSearch
  (bind _returnvalue (Game|Player|GetPlayerPawn 0))
  (bind _sightarrow (Variables|Default|GetSightArrow))
  (bind _returnvalue_2 (Transformation|GetWorldLocation _sightarrow))
  (bind _returnvalue_3 (Transformation|GetActorLocation _returnvalue))
  ;[1 1 1] Visual Search for targets: if target is lost return to search state, if target is seen enter approach state
  (if (<= (Math|Vector|VectorLength (- _returnvalue_2 _returnvalue_3)) (Variables|Default|GetVisualSearchRadius))
    (bind _returnvalue_4 (Collision|LineTraceByChannel _returnvalue_2 _returnvalue_3 "TraceTypeQuery1" false 0 "None"))
    (if _returnvalue_4
      (Variables|Default|SetTargetVisible false)
      (else
        (Variables|Default|SetTargetVisible true)))))

(fn AdjustRotationtoTarget
  (Variables|Default|SetIsAiming true))

(fn TargetRangeCheck)