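; Humanoid AI character Blueprint, an unfinished state-driven enemy meant to wander, spot the player and fight with an attached AlienGun.
; BrainTick runs VisualSearch in Search state, using distance and line-of-sight traces to switch to Approach or move to the player's location on losing sight.
; Startup, timer, wandering, death, range-check and projectile logic is disconnected, leaving BeginPlay, Tick and ShootAtTarget empty.
; DamageActor subtracts zero health, and Approach only sets the state.
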(event OnComponentBeginOverlap(Collision)
  (params (OverlappedComponent :type Primitive%20Component%20Object%20Reference) (OtherActor :type Actor%20Object%20Reference) (OtherComp :type Primitive%20Component%20Object%20Reference) (OtherBodyIndex :type Integer) (bFromSweep :type Boolean) (SweepResult :type Hit%20Result%20Structure%20%28by%20ref%29))
  ;[1 1 1] Death on Overlap
)

(event Custom|EnemyBecameVisible
  ;[1 1 1] When enemy is seen enter approach state, choose approach point, move to
  (Variables|Default|SetAIState "NewEnumerator1"))

(event Custom|EnemyLost
  ;[1 1 1] EnemyLostEvent
  (Variables|Default|SetAIState "NewEnumerator0")
  (Variables|/Script/Engine.CharacterMovementComponent|SetMaxWalkSpeed (Variables|Character|GetCharacterMovement) (Variables|Default|GetWalkSpeed))
  (bind _output_get (Variables|Default|SetTargetLastLocation (Transformation|GetActorLocation (Game|Player|GetPlayerPawn 0))))
  (AI|AIMoveTo self _output_get 0 5.0 false
    (:then
      (Variables|Default|SetIsMoving true))
    (:OnSuccess
      (Variables|Default|SetIsMoving false :!label _label)
      (Variables|/Script/Engine.CharacterMovementComponent|SetMaxWalkSpeed (Variables|Character|GetCharacterMovement) (Variables|Default|GetStandingSpeed)))
    (:OnFail
      (goto _label))))

(event Custom|DamageActor
  ;[1 1 1] Take Damage
  (Variables|Default|SetHealth (- (Variables|Default|GetHealth) (Math|Conversions|ToFloat(Integer) 0)))
  (Development|PrintString "damaged"))

(event EventBeginPlay
  ;[1 1 1] Begin Play Events
)

(event EventTick
  (params (DeltaSeconds :type Float%20%28single-precision%29))
  ;[1 1 1] Tick events
)

(fn ConstructionScript)

(fn BrainTick
  (switch Utilities|FlowControl|Switch|SwitchonHumanoiAIState (Variables|Default|GetAIState)
    (:NewEnumerator0
      (CallFunction|VisualSearch))))

(fn ShootatTarget)

(fn VisualSearch
  (bind _returnvalue (Game|Player|GetPlayerPawn 0))
  (bind _sightarrow (Variables|Default|GetSightArrow))
  (bind _returnvalue_2 (Transformation|GetWorldLocation _sightarrow))
  (bind _returnvalue_3 (Transformation|GetActorLocation _returnvalue))
  ;[1 1 1] Visual Search for targets: if target is lost return to search state, if target is seen enter approach state
  (if (<= (Math|Vector|VectorLength (- _returnvalue_2 _returnvalue_3)) (Variables|Default|GetVisualSearchRadius))
    (bind _returnvalue_4 (Collision|LineTraceByChannel _returnvalue_2 _returnvalue_3 "TraceTypeQuery1" false 0 "None"))
    (if _returnvalue_4
      (Variables|Default|SetTargetVisible false)
      (CallFunction|EnemyLost)
      (else
        (Variables|Default|SetTargetVisible true)
        (CallFunction|EnemyBecameVisible)))))

(fn AdjustRotationtoTarget
  (Variables|Default|SetIsAiming true))

(fn TargetRangeCheck)