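; Spawner Blueprint for RCTA Pilot Scenario 1 that prepares spawn and destination data for nine spawn points.
; On BeginPlay it pairs two groups, giving Spawn1–4 the world locations of Spawn5–9 as destinations and vice versa.
; It also fills hard-coded index sequences for spawn order and for picks from four- or five-entry destination lists.
; No logic here consumes this data, as SpawnActor, Tick and the construction script are empty.
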(event EventBeginPlay
  (Utilities|FlowControl|Sequence
    (:then_0
      (Variables|Default|SetDestinations_Spawn1 (Utilities|Array|MakeArray (Transformation|GetWorldLocation (Variables|Default|GetSpawn5)) (Transformation|GetWorldLocation (Variables|Default|GetSpawn6)) (Transformation|GetWorldLocation (Variables|Default|GetSpawn7)) (Transformation|GetWorldLocation (Variables|Default|GetSpawn8)) (Transformation|GetWorldLocation (Variables|Default|GetSpawn9))))
      (Variables|Default|SetDestinations_Spawn2 (Utilities|Array|MakeArray (Transformation|GetWorldLocation (Variables|Default|GetSpawn5)) (Transformation|GetWorldLocation (Variables|Default|GetSpawn6)) (Transformation|GetWorldLocation (Variables|Default|GetSpawn7)) (Transformation|GetWorldLocation (Variables|Default|GetSpawn8)) (Transformation|GetWorldLocation (Variables|Default|GetSpawn9))))
      (Variables|Default|SetDestinations_Spawn3 (Utilities|Array|MakeArray (Transformation|GetWorldLocation (Variables|Default|GetSpawn5)) (Transformation|GetWorldLocation (Variables|Default|GetSpawn6)) (Transformation|GetWorldLocation (Variables|Default|GetSpawn7)) (Transformation|GetWorldLocation (Variables|Default|GetSpawn8)) (Transformation|GetWorldLocation (Variables|Default|GetSpawn9))))
      (Variables|Default|SetDestinations_Spawn4 (Utilities|Array|MakeArray (Transformation|GetWorldLocation (Variables|Default|GetSpawn5)) (Transformation|GetWorldLocation (Variables|Default|GetSpawn6)) (Transformation|GetWorldLocation (Variables|Default|GetSpawn7)) (Transformation|GetWorldLocation (Variables|Default|GetSpawn8)) (Transformation|GetWorldLocation (Variables|Default|GetSpawn9))))
      (Variables|Default|SetDestinations_Spawn5 (Utilities|Array|MakeArray (Transformation|GetWorldLocation (Variables|Default|GetSpawn1)) (Transformation|GetWorldLocation (Variables|Default|GetSpawn2)) (Transformation|GetWorldLocation (Variables|Default|GetSpawn3)) (Transformation|GetWorldLocation (Variables|Default|GetSpawn4))))
      (Variables|Default|SetDestinations_Spawn6 (Utilities|Array|MakeArray (Transformation|GetWorldLocation (Variables|Default|GetSpawn1)) (Transformation|GetWorldLocation (Variables|Default|GetSpawn2)) (Transformation|GetWorldLocation (Variables|Default|GetSpawn3)) (Transformation|GetWorldLocation (Variables|Default|GetSpawn4))))
      (Variables|Default|SetDestinations_Spawn7 (Utilities|Array|MakeArray (Transformation|GetWorldLocation (Variables|Default|GetSpawn1)) (Transformation|GetWorldLocation (Variables|Default|GetSpawn2)) (Transformation|GetWorldLocation (Variables|Default|GetSpawn3)) (Transformation|GetWorldLocation (Variables|Default|GetSpawn4))))
      (Variables|Default|SetDestinations_Spawn8 (Utilities|Array|MakeArray (Transformation|GetWorldLocation (Variables|Default|GetSpawn1)) (Transformation|GetWorldLocation (Variables|Default|GetSpawn2)) (Transformation|GetWorldLocation (Variables|Default|GetSpawn3)) (Transformation|GetWorldLocation (Variables|Default|GetSpawn4))))
      (Variables|Default|SetDestinations_Spawn9 (Utilities|Array|MakeArray (Transformation|GetWorldLocation (Variables|Default|GetSpawn1)) (Transformation|GetWorldLocation (Variables|Default|GetSpawn2)) (Transformation|GetWorldLocation (Variables|Default|GetSpawn3)) (Transformation|GetWorldLocation (Variables|Default|GetSpawn4)))))
    (:then_1
      (Variables|Default|SetSpawnCycle_Array1 (Utilities|Array|MakeArray (Variables|Default|Get0) (Variables|Default|Get4) (Variables|Default|Get5) (Variables|Default|Get2) (Variables|Default|Get1) (Variables|Default|Get3) (Variables|Default|Get2) (Variables|Default|Get1) (Variables|Default|Get3) (Variables|Default|Get4) (Variables|Default|Get0) (Variables|Default|Get5)))
      (Variables|Default|SetSpawnCycle_Array2 (Utilities|Array|MakeArray (Variables|Default|Get4) (Variables|Default|Get2) (Variables|Default|Get5) (Variables|Default|Get0) (Variables|Default|Get3) (Variables|Default|Get1) (Variables|Default|Get0) (Variables|Default|Get2) (Variables|Default|Get1) (Variables|Default|Get3) (Variables|Default|Get4) (Variables|Default|Get5))))
    (:then_2
      (Variables|Default|SetDestinationCycle_4_Array1 (Utilities|Array|MakeArray (Variables|Default|Get2) (Variables|Default|Get0) (Variables|Default|Get3) (Variables|Default|Get1) (Variables|Default|Get3) (Variables|Default|Get0) (Variables|Default|Get1) (Variables|Default|Get2) (Variables|Default|Get0) (Variables|Default|Get3) (Variables|Default|Get1) (Variables|Default|Get2)))
      (Variables|Default|SetDestinationCycle_5_Array1 (Utilities|Array|MakeArray (Variables|Default|Get0) (Variables|Default|Get1) (Variables|Default|Get3) (Variables|Default|Get4) (Variables|Default|Get2) (Variables|Default|Get3) (Variables|Default|Get0) (Variables|Default|Get4) (Variables|Default|Get1) (Variables|Default|Get2) (Variables|Default|Get4) (Variables|Default|Get2))))))

(event EventTick
  (params (DeltaSeconds :type Float%20%28single-precision%29)))

(fn ConstructionScript)

(fn SpawnActor)