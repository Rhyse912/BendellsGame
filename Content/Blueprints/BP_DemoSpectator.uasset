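; Demo spectator player controller that provides the in-game main menu overlay.
; On BeginPlay, where cosmetic events can run and the controller is local, it replaces any existing menu widget with a new MainMenuScreen, collapsed and faded out.
; The InGameMenu input toggles the menu through its fade-in and fade-out, tracked by ShowingMainMenu, and is ignored on maps whose name ends in EntryMap.
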(event EventBeginPlay
  (Networking|CanExecuteCosmeticEvents
    (:True
      (if (Pawn|IsLocalPlayerController)
        (Utilities|IsValid (Variables|Default|GetMainMenu)
          (:Is%20Valid
            (Widget|RemovefromParent (Variables|Default|GetMainMenu)))
          (:Is%20Not%20Valid
            _))
        (bind _returnvalue (UserInterface|CreateWidget "/Game/Squad/Content/UI/Widgets/MainMenuScreen.MainMenuScreen_C" self))
        (Variables|Default|SetMainMenu _returnvalue)
        (UserInterface|Viewport|AddtoViewport _returnvalue 0)
        (Widget|SetVisibility (Variables|Default|GetMainMenu) "Collapsed")
        (Default|BeginFadeOut (Variables|Default|GetMainMenu))
        (Variables|Default|SetbShowingMainMenu false)))))

(event Input|ActionEvents|InputActionInGameMenu
  (params (Key :type Key%20Structure :default "AnyKey"))
  (bind _mainmenu (Variables|Default|GetMainMenu))
  (:Pressed
    (if (not (Utilities|String|EndsWith (CallFunction|GetCurrentMapName) "EntryMap" "CaseSensitive"))
      (if (Variables|Default|GetbShowingMainMenu)
        (Default|BeginFadeOut _mainmenu)
        (Variables|Default|SetbShowingMainMenu false)
        (else
          (Default|BeginFadein _mainmenu)
          (Variables|Default|SetbShowingMainMenu true))))))

(fn ConstructionScript)