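; BP_FTEManager is the Blueprint manager for first-time event (FTE) prompts, extending the parent's ShowGenericFTE event.
; After the parent call, it checks the user's ShowFTE setting and branches on FTE name, but its only case is an empty example.
; A template function, never called, shows a toast to a valid controller with action keys formatted into the text.
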(event EventShowGenericFTE
  (params (Controller :type SQ%20Player%20Controller%20Object%20Reference) (FTEName :type Name))
  (|CallParentFunction Controller FTEName)
  (if (Variables|/Script/Squad.SQGameUserSettings|GetbShowFTE (Class|SQBlueprintLibrary|GetSquadGameUserSettings))
    (if (Utilities|Name|Equal(Name) FTEName "fteshowexamplefunction")
      _)))

(fn ExampleFTEFunction
  (params (Controller :type SQ%20Player%20Controller%20Object%20Reference))
  (bind _examplevariable (Variables|Default|GetExampleVariable))
  (bind (_ftetext _actionkeys _lifetime) (Utilities|Struct|BreakSQFTEText _examplevariable))
  (Utilities|IsValid Controller
    (:Is%20Valid
      (Class|SQPlayerController|ShowToast Controller (Class|SQBlueprintLibrary|FormatTextActionKeys _ftetext _actionkeys) _lifetime false))))