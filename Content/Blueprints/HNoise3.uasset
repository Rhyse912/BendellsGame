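; HNoise3 is an AI pawn that walks to an assigned destination and destroys itself on arrival.
; It starts moving one second after BeginPlay; when stalled, Tick sends it to a random nearby navigable point, then back toward the destination.
; Marking it swaps a body material to emissive for two seconds.
; Player-sight functions set visibility flags but nothing here calls BrainTick, and the shooting logic is empty or disconnected.
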(event EventBeginPlay
  ;[1 1 1] Begin play events
  (Utilities|FlowControl|Sequence
    (:then_4
      ;;[1 1 1] Delay for 1 second and then proceed to destination
      (Utilities|FlowControl|Delay 1.0)
      (Variables|/Script/Engine.CharacterMovementComponent|SetMaxWalkSpeed (Variables|Character|GetCharacterMovement) (Variables|Default|GetMovementSpeed))
      (Variables|Default|SetIsMoving true)
      (AI|AIMoveTo self (Variables|Default|GetDestination) 0 5e+02 false
        (:OnSuccess
          (Actor|DestroyActor))))))

(event EventOnMarkTarget
  ;[1 1 1] Tick events
  (Rendering|Material|SetMaterial (Variables|Character|GetMesh) 2 "/Game/Mixamo/Body_MATEmmisive.Body_MATEmmisive")
  (Utilities|Time|SetTimerbyFunctionName 0 "RemoveHighlighting" 2.0))

(event EventTick
  (params (DeltaSeconds :type Float%20%28single-precision%29))
  (bind _self self)
  ;[1 1 1] Tick events
  (if (and (<= (Math|Vector|VectorLength (Variables|/Script/Engine.MovementComponent|GetVelocity (Variables|Character|GetCharacterMovement))) 0.0) (Variables|Default|GetIsMoving))
    (Components|Movement|StopMovementImmediately (Variables|Character|GetCharacterMovement))
    (AI|AIMoveTo _self (.RandomLocation (Class|NavigationSystem|GetRandomPointinNavigableRadius (Transformation|GetWorldLocation (Variables|Collision|GetCapsuleComponent)) 2e+02)) 0 25.0 false
      (:OnSuccess
        (AI|AIMoveTo _self (Variables|Default|GetDestination) 0 5e+02 false
          (:OnSuccess
            (Actor|DestroyActor)))))))

(event EventAssignDestination
  (params (Destination :type Vector))
  ;[1 1 1] Begin play events
  ;;[1 1 1] Accept destination
  (Variables|Default|SetDestination Destination))

(fn ConstructionScript)

(fn BrainTick
  (switch Utilities|FlowControl|Switch|SwitchonHumanoiAIState (Variables|Default|GetAIState)
    (:NewEnumerator0
      (CallFunction|VisualSearch))))

(fn ShootatTarget)

(fn VisualSearch
  (bind _returnvalue (Game|Player|GetPlayerPawn 0))
  (bind _sightarrow (Variables|Default|GetSightArrow))
  (bind _returnvalue_2 (Transformation|GetWorldLocation _sightarrow))
  (bind _returnvalue_3 (Transformation|GetActorLocation _returnvalue))
  ;[1 1 1] Visual Search for targets: if target is lost return to search state, if target is seen enter approach state
  (if (<= (Math|Vector|VectorLength (- _returnvalue_2 _returnvalue_3)) (Variables|Default|GetVisualSearchRadius))
    (bind _returnvalue_4 (Collision|LineTraceByChannel _returnvalue_2 _returnvalue_3 "TraceTypeQuery1" false 0 "None"))
    (if _returnvalue_4
      (Variables|Default|SetTargetVisible false)
      (else
        (Variables|Default|SetTargetVisible true)))))

(fn AdjustRotationtoTarget
  (Variables|Default|SetIsAiming true))

(fn TargetRangeCheck)

(fn RemoveHighlighting
  (Rendering|Material|SetMaterial (Variables|Character|GetMesh) 2 "/Game/Mixamo/Blu_Body_MAT.Blu_Body_MAT"))