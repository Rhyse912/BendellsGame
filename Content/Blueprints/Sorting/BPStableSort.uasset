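; BPStableSort is a reusable sorting Blueprint with a helper for ordering UI grid widgets.
; Sort rebuilds the passed array by insertion sort, placing each element before the first one for which SortImplementation returns false, otherwise at the end.
; SortImplementation is a placeholder comparison that always returns false, so on its own Sort reverses the input.
; SortUIGridElements sets each valid grid slot's row to its array index.
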(fn SortImplementation
  (params (Object :type Object%20Object%20Reference) (OtherObject :type Object%20Object%20Reference))
  (return false))

(fn Sort
  (params (SortingArray :type Array%20of%20Object%20Object%20References))
  (bind _sortedarrayresult (LocalVariables|GetSortedArrayResult))
  (for (_array_element _array_index) SortingArray
    (if (== _array_index 0)
      (Utilities|Array|Add (LocalVariables|GetSortedArrayResult) _array_element)
      (else
        (LocalVariables|SetInserted false)
        (bind (_array_element_2 _array_index_2) (Utilities|Array|ForEachLoopwithBreak _sortedarrayresult :!label _label)
          (:LoopBody
            (if (not (CallFunction|SortImplementation _array_element _array_element_2))
              (Utilities|Array|Insert (LocalVariables|GetSortedArrayResult) _array_element _array_index_2)
              (LocalVariables|SetInserted true)
              (goto _label Break)))
          (:Completed
            (if (not (LocalVariables|GetInserted)) ; If nothing was found then the tested object is the largest in the set
              (Utilities|Array|Insert (LocalVariables|GetSortedArrayResult) _array_element (Utilities|Array|Length _sortedarrayresult))))))))
  (Utilities|Array|Clear SortingArray)
  (Utilities|Array|AppendArray SortingArray (LocalVariables|GetSortedArrayResult)))

(fn SortUIGridElements
  (params (SortedArray :type Array%20of%20Widget%20Object%20References))
  (for (_array_element _array_index) SortedArray
    (Utilities|IsValid (Class|WidgetLayoutLibrary|SlotasGridSlot _array_element)
      (:Is%20Valid
        (Class|GridSlot|SetRow (Class|WidgetLayoutLibrary|SlotasGridSlot _array_element) _array_index)))))