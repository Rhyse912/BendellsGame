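; HTarget1RT is a short-lived AI character target that destroys itself three seconds after BeginPlay.
; Marking it temporarily swaps a body material to an emissive highlight, with a timer restoring the red one.
; BrainTick, not called in this graph, runs a distance and line-trace check for player visibility in the Search state.
; Movement, weapon spawning and shooting-range logic are disconnected, and the shooting functions are stubs.
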(event EventBeginPlay
  ;[1 1 1] Begin play events
  (Utilities|FlowControl|Delay 3.0)
  (Actor|DestroyActor))

(event EventOnMarkTarget
  ;[1 1 1] Tick events
  (Rendering|Material|SetMaterial (Variables|Character|GetMesh) 2 "/Game/Mixamo/Body_MATEmmisive.Body_MATEmmisive")
  (Utilities|Time|SetTimerbyFunctionName 0 "RemoveHighlighting" 2.0))

(event EventTick
  (params (DeltaSeconds :type Float%20%28single-precision%29))
  ;[1 1 1] Tick events
)

(event EventAssignDestination
  (params (Destination :type Vector))
  ;[1 1 1] Begin play events
  ;;[1 1 1] Accept destination
  (Variables|Default|SetDestination Destination))

(fn ConstructionScript)

(fn BrainTick
  (switch Utilities|FlowControl|Switch|SwitchonHumanoiAIState (Variables|Default|GetAIState)
    (:NewEnumerator0
      (CallFunction|VisualSearch))))

(fn ShootatTarget)

(fn VisualSearch
  (bind _returnvalue (Game|Player|GetPlayerPawn 0))
  (bind _sightarrow (Variables|Default|GetSightArrow))
  (bind _returnvalue_2 (Transformation|GetWorldLocation _sightarrow))
  (bind _returnvalue_3 (Transformation|GetActorLocation _returnvalue))
  ;[1 1 1] Visual Search for targets: if target is lost return to search state, if target is seen enter approach state
  (if (<= (Math|Vector|VectorLength (- _returnvalue_2 _returnvalue_3)) (Variables|Default|GetVisualSearchRadius))
    (bind _returnvalue_4 (Collision|LineTraceByChannel _returnvalue_2 _returnvalue_3 "TraceTypeQuery1" false 0 "None"))
    (if _returnvalue_4
      (Variables|Default|SetTargetVisible false)
      (else
        (Variables|Default|SetTargetVisible true)))))

(fn AdjustRotationtoTarget
  (Variables|Default|SetIsAiming true))

(fn TargetRangeCheck)

(fn RemoveHighlighting
  (Rendering|Material|SetMaterial (Variables|Character|GetMesh) 2 "/Game/Mixamo/Red_Body_MAT.Red_Body_MAT"))