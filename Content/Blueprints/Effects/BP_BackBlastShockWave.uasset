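; BP_BackBlastShockWave is an effect Blueprint that creates a back-blast shockwave when its Explode event fires.
; BackBlastShockWave casts a ring of evenly spaced traces, one per HorizontalSteps, forming a fixed-length cone around the actor's local up axis.
; Each trace goes to SpawnEmitterAtTraceIntersect with the Instigator, which by its name places emitters where the traces hit surfaces.
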(event EventExplode
  (params (Instigator :type Actor%20Object%20Reference))
  (CallFunction|BackBlastShockWave Instigator))

(fn ConstructionScript
  (|CallParentFunction))

(fn BackBlastShockWave
  (params (Instigator :type Actor%20Object%20Reference))
  (bind _returnvalue (Transformation|GetActorLocation))
  (for _index (range 1 (Variables|Default|GetHorizontalSteps))
    (CallFunction|SpawnEmitteratTraceIntersect _returnvalue (+ _returnvalue (Math|Vector|RotateVector (Math|Vector|MakeVector 6.5e+02 0.0 0.0) (Math|Rotator|CombineRotators (Math|Rotator|MakeRotator 0.0 65.0 (* _index (/ 3.6e+02 (Math|Conversions|ToFloat(Integer) (Variables|Default|GetHorizontalSteps))))) (Transformation|GetActorRotation)))) Instigator)))