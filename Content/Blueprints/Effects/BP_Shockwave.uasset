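; Shockwave effect actor that scatters a particle emitter across the surrounding surfaces when Explode is called.
; Explode fires fixed-length line traces from just above the actor in a spherical fan, set by horizontal and vertical step counts.
; Vertical steps become a loop range symmetric about the horizon.
; Each visibility trace ignores the instigator and, on a hit, spawns the emitter aligned to the impact normal.
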(event EventBeginPlay)

(event Collision|EventActorBeginOverlap
  (params (OtherActor :type Actor%20Object%20Reference)))

(event EventTick
  (params (DeltaSeconds :type Float%20%28single-precision%29)))

(fn ConstructionScript)

(fn Explode
  (params (Instigator :type Actor%20Object%20Reference))
  (bind _returnvalue (Transformation|GetActorLocation))
  (bind (_x _y _z) (Math|Vector|BreakVector _returnvalue))
  (bind _returnvalue_2 (+ _z 1e+02))
  (bind _returnvalue_3 (Math|Vector|MakeVector _x _y _returnvalue_2))
  (bind (_positiveint _negativeint) (CallFunction|ConvertStepstoLoops (Variables|Default|GetVerticalSteps)))
  (for _index (range 1 (Variables|Default|GetHorizontalSteps))
    (for _index_2 (range _negativeint _positiveint)
      (CallFunction|SpawnEmitteratTraceIntersect _returnvalue_3 (+ _returnvalue_3 (Math|Vector|RotateVector (Math|Vector|MakeVector 6.5e+02 0.0 0.0) (Math|Rotator|MakeRotator 0.0 (* _index_2 (Math|Conversions|ToFloat(Integer) (/ 180 (+ (Variables|Default|GetVerticalSteps) 1)))) (* _index (/ 3.6e+02 (Math|Conversions|ToFloat(Integer) (Variables|Default|GetHorizontalSteps))))))) Instigator))))

(fn ConvertStepstoLoops
  (params (Steps :type Integer :default 0))
  (if (== (Math|Integer|%(Integer) Steps 2) 1)
    _
    (else
      (Variables|Default|SetVerticalSteps (- Steps 1))))
  (return (/ Steps 2) (/ Steps -2)))

(fn SpawnEmitteratTraceIntersect
  (params (StartTrace :type Vector) (EndTrace :type Vector) (Instigator :type Actor%20Object%20Reference))
  (bind (_outhit _returnvalue) (Collision|LineTraceByChannel StartTrace EndTrace "TraceTypeQuery1" false (Utilities|Array|MakeArray Instigator) "None"))
  (if _returnvalue
    (Effects|SpawnEmitteratLocation (Variables|Default|GetEmitter%20Being%20Played) (.Location (Collision|BreakHitResult _outhit)) (Math|Conversions|RotationFromXVector (.ImpactNormal (Collision|BreakHitResult _outhit))))
    (return)
    (else
      (return))))