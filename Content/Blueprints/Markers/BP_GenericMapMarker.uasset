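; Generic map marker that is shown on the HUD for players in the same team and squad as its owner.
; On dedicated, listen or standalone servers, construction copies the owner's team and squad IDs onto the marker.
; BeginPlay registers it in squad PlayerStates on dedicated servers, otherwise in the relevant local PlayerState and HUD, after a short delay on listen/standalone.
; Destruction unregisters it only on listen/standalone.
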(event Custom|SetTexture
  (params (Texture :type Texture%202D%20Object%20Reference))
  (Variables|Default|SetTexture (Variables|Default|GetMapIcon) Texture))

(event EventDestroyed
  (bind _returnvalue (Game|GetPlayerController 0))
  (if (not (Networking|IsDedicatedServer))
    (if (CallFunction|IsStandaloneorListenServer)
      (Utilities|IsValid _returnvalue
        (:Is%20Valid
          (bind _assqplayer_state (Utilities|Casting|CastTo (Variables|/Script/Engine.Controller|GetPlayerState _returnvalue)))
          (Utilities|Array|RemoveItem (Variables|Default|GetRelevantMapMarkers _assqplayer_state) self))))))

(event EventBeginPlay
  (bind _returnvalue (Game|GetPlayerController 0))
  (Variables|Default|SetTint (Variables|Default|GetMapIcon) (Variables|Default|GetDefaultTint))
  (if (Networking|IsDedicatedServer)
    (bind _assqplayer_controller (Utilities|Casting|CastTo (Components|GetOwner))) ; Register markers in the server playerstates
    (Utilities|IsValid (Variables|Default|GetSquadState _assqplayer_controller)
      (:Is%20Valid
        (for _array_element (Variables|Default|GetPlayerStates (Variables|Default|GetSquadState _assqplayer_controller))
          (bind _assqplayer_controller_2 (Utilities|Casting|CastTo (Components|GetOwner)))
          (bind _isrelevant (CallFunction|MarkerIsSquadandTeamRelevant _assqplayer_controller_2))
          (if _isrelevant
            (Utilities|Array|Add (Variables|Default|GetRelevantMapMarkers _array_element) self)))))
    (else
      (if (CallFunction|IsStandaloneorListenServer) ; Register markers on the client
        (Utilities|FlowControl|Delay 0.1) ; Allow proper initialization of the marker in the creation code
      )
      (bind _assqplayer_controller_3 (Utilities|Casting|CastTo _returnvalue))
      (bind _assqplayer_state (Utilities|Casting|CastTo (Variables|/Script/Engine.Controller|GetPlayerState _returnvalue)))
      (bind _isrelevant_2 (CallFunction|MarkerIsSquadandTeamRelevant _returnvalue)) ; Check relevancy
      (if _isrelevant_2
        (Utilities|Array|Add (Variables|Default|GetRelevantMapMarkers _assqplayer_state) self)
        (bind _asbp_hud (Utilities|Casting|CastTo (HUD|GetHUD _assqplayer_controller_3)))
        (CallFunction|ShowMarkeronHudEvent _asbp_hud self) ; Show on hud
      ))))

(fn ConstructionScript
  (if (Networking|IsDedicatedServer)
    (bind _assqplayer_controller (Utilities|Casting|CastTo (Components|GetOwner) :!label _label))
    (CallFunction|SetTeam (Utilities|Enum|ByteToEnumObject (Math|Conversions|ToByte(Integer) (Variables|Default|GetId (Variables|Default|GetTeamState _assqplayer_controller)))))
    (Utilities|IsValid (Variables|Default|GetSquadState _assqplayer_controller)
      (:Is%20Valid
        (CallFunction|SetSquad (Variables|Default|GetId (Variables|Default|GetSquadState _assqplayer_controller)))))
    (elif (CallFunction|IsStandaloneorListenServer)
      (goto _label))))

(fn MarkerIsSquadandTeamRelevant
  (params (Controller :type Controller%20Object%20Reference))
  (bind _assqplayer_controller (Utilities|Casting|CastTo Controller)
    (:then
      (bind _assqplayer_state (Utilities|Casting|CastTo (Variables|/Script/Engine.Controller|GetPlayerState Controller))
        (:then
          (Utilities|IsValid (Variables|Default|GetSquadState _assqplayer_state)
            (:Is%20Valid
              (return (and (== (Variables|Default|GetSquad) (Variables|Default|GetId (Variables|Default|GetSquadState _assqplayer_state))) (== (Math|Conversions|ToByte(Integer) (Variables|Default|GetId (Variables|Default|GetTeamState _assqplayer_controller))) (Variables|Default|GetTeam)))))
            (:Is%20Not%20Valid
              _)))
        (:CastFailed
          _)))
    (:CastFailed
      _))
  (return false))