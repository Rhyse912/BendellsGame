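; Timed humanoid spawner that fixes itself at a set world position and sends out AI target and noise pawns.
; A looping timer calls SpawnTarget, which picks the pawn type from CycleArray and spawns it at the navmesh-projected spawn point.
; AssignDestinationFromID messages each pawn its destination for HSpawn1, then advances SpawnIndex, which resets once past ArraySize.
; Non-humanoid spawn and destination branches remain but are disconnected.
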(event EventBeginPlay
  (bind _defaultsceneroot (Variables|Default|GetDefaultSceneRoot))
  (Utilities|FlowControl|Sequence
    (:then_0
      ;[1 1 1] SetWorld location and rotation
      (Transformation|SetWorldLocation _defaultsceneroot "1000.000000,1500.000000, 0" false false)
      (Transformation|SetWorldRotation _defaultsceneroot "0,0.000000, 0" false false))
    (:then_1
      ;[1 1 1] Begin spawn loop, cycle every X seconds
      (Utilities|Time|SetTimerbyFunctionName 0 "SpawnTarget" (Variables|Default|GetSpawnLoopTimer) true))
    (:then_2
      ;[1 1 1] Choose SpawnID
      (Variables|Default|SetSpawnerID "NewEnumerator4")
      (Variables|Default|SetCycleArray (Variables|Default|GetHTargetCycleArray1)))
    (:then_3
      ;[1 1 1] Target Destination Points
      (Variables|Default|SetDestinationArray1 (Utilities|Array|MakeArray (Variables|Default|GetSpawnLocation4) (Variables|Default|GetSpawnLocation2) (Variables|Default|GetSpawnLocation3) (Variables|Default|GetSpawnLocation4) (Variables|Default|GetSpawnLocation3) (Variables|Default|GetSpawnLocation2) (Variables|Default|GetSpawnLocation3) (Variables|Default|GetSpawnLocation4) (Variables|Default|GetSpawnLocation2) (Variables|Default|GetSpawnLocation2) (Variables|Default|GetSpawnLocation3) (Variables|Default|GetSpawnLocation4) (Variables|Default|GetSpawnLocation4) (Variables|Default|GetSpawnLocation2) (Variables|Default|GetSpawnLocation3)))
      (Variables|Default|SetDestinationArray2 (Utilities|Array|MakeArray (Variables|Default|GetSpawnLocation1) (Variables|Default|GetSpawnLocation4) (Variables|Default|GetSpawnLocation3) (Variables|Default|GetSpawnLocation4) (Variables|Default|GetSpawnLocation1) (Variables|Default|GetSpawnLocation3) (Variables|Default|GetSpawnLocation3) (Variables|Default|GetSpawnLocation4) (Variables|Default|GetSpawnLocation1) (Variables|Default|GetSpawnLocation1) (Variables|Default|GetSpawnLocation3) (Variables|Default|GetSpawnLocation4) (Variables|Default|GetSpawnLocation1) (Variables|Default|GetSpawnLocation4) (Variables|Default|GetSpawnLocation3)))
      (Variables|Default|SetDestinationArray3 (Utilities|Array|MakeArray (Variables|Default|GetSpawnLocation1) (Variables|Default|GetSpawnLocation2) (Variables|Default|GetSpawnLocation1) (Variables|Default|GetSpawnLocation4) (Variables|Default|GetSpawnLocation1) (Variables|Default|GetSpawnLocation2) (Variables|Default|GetSpawnLocation1) (Variables|Default|GetSpawnLocation4) (Variables|Default|GetSpawnLocation1) (Variables|Default|GetSpawnLocation2) (Variables|Default|GetSpawnLocation1) (Variables|Default|GetSpawnLocation4) (Variables|Default|GetSpawnLocation1) (Variables|Default|GetSpawnLocation2) (Variables|Default|GetSpawnLocation4)))
      (Variables|Default|SetDestinationArray4 (Utilities|Array|MakeArray (Variables|Default|GetSpawnLocation1) (Variables|Default|GetSpawnLocation2) (Variables|Default|GetSpawnLocation3) (Variables|Default|GetSpawnLocation2) (Variables|Default|GetSpawnLocation1) (Variables|Default|GetSpawnLocation2) (Variables|Default|GetSpawnLocation3) (Variables|Default|GetSpawnLocation2) (Variables|Default|GetSpawnLocation1) (Variables|Default|GetSpawnLocation2) (Variables|Default|GetSpawnLocation3) (Variables|Default|GetSpawnLocation2) (Variables|Default|GetSpawnLocation1) (Variables|Default|GetSpawnLocation2) (Variables|Default|GetSpawnLocation3)))
      (Variables|Default|SetHDestinationArray1 (Utilities|Array|MakeArray (Variables|Default|GetHSpawnLocation2) (Variables|Default|GetHSpawnLocation2) (Variables|Default|GetHSpawnLocation2) (Variables|Default|GetHSpawnLocation2) (Variables|Default|GetHSpawnLocation2) (Variables|Default|GetHSpawnLocation2) (Variables|Default|GetHSpawnLocation2) (Variables|Default|GetHSpawnLocation2) (Variables|Default|GetHSpawnLocation2) (Variables|Default|GetHSpawnLocation2) (Variables|Default|GetHSpawnLocation2) (Variables|Default|GetHSpawnLocation2) (Variables|Default|GetHSpawnLocation2) (Variables|Default|GetHSpawnLocation2) (Variables|Default|GetHSpawnLocation2)))
      (Variables|Default|SetHDestinationArray2 (Utilities|Array|MakeArray (Variables|Default|GetHSpawnLocation1) (Variables|Default|GetHSpawnLocation1) (Variables|Default|GetHSpawnLocation1) (Variables|Default|GetHSpawnLocation1) (Variables|Default|GetHSpawnLocation1) (Variables|Default|GetHSpawnLocation1) (Variables|Default|GetHSpawnLocation1) (Variables|Default|GetHSpawnLocation1) (Variables|Default|GetHSpawnLocation1) (Variables|Default|GetHSpawnLocation1) (Variables|Default|GetHSpawnLocation1) (Variables|Default|GetHSpawnLocation1) (Variables|Default|GetHSpawnLocation1) (Variables|Default|GetHSpawnLocation1) (Variables|Default|GetHSpawnLocation1)))
      (Variables|Default|SetHDestinationArray3 (Utilities|Array|MakeArray (Variables|Default|GetHSpawnLocation4) (Variables|Default|GetHSpawnLocation4) (Variables|Default|GetHSpawnLocation4) (Variables|Default|GetHSpawnLocation4) (Variables|Default|GetHSpawnLocation4) (Variables|Default|GetHSpawnLocation4) (Variables|Default|GetHSpawnLocation4) (Variables|Default|GetHSpawnLocation4) (Variables|Default|GetHSpawnLocation4) (Variables|Default|GetHSpawnLocation4) (Variables|Default|GetHSpawnLocation4) (Variables|Default|GetHSpawnLocation4) (Variables|Default|GetHSpawnLocation4) (Variables|Default|GetHSpawnLocation4) (Variables|Default|GetHSpawnLocation4)))
      (Variables|Default|SetHDestinationArray4 (Utilities|Array|MakeArray (Variables|Default|GetHSpawnLocation3) (Variables|Default|GetHSpawnLocation3) (Variables|Default|GetHSpawnLocation3) (Variables|Default|GetHSpawnLocation3) (Variables|Default|GetHSpawnLocation3) (Variables|Default|GetHSpawnLocation3) (Variables|Default|GetHSpawnLocation3) (Variables|Default|GetHSpawnLocation3) (Variables|Default|GetHSpawnLocation3) (Variables|Default|GetHSpawnLocation3) (Variables|Default|GetHSpawnLocation3) (Variables|Default|GetHSpawnLocation3) (Variables|Default|GetHSpawnLocation3) (Variables|Default|GetHSpawnLocation3) (Variables|Default|GetHSpawnLocation3))))))

(fn ConstructionScript)

(fn SpawnTarget
  (bind _spawn (Variables|Default|GetSpawn))
  (bind _spawn_2 (Variables|Default|GetSpawn))
  (bind _spawn_3 (Variables|Default|GetSpawn))
  (bind _returnvalue (Transformation|GetWorldLocation _spawn))
  (bind _returnvalue_2 (Transformation|GetWorldLocation _spawn_2))
  (bind _returnvalue_3 (Transformation|GetWorldLocation _spawn_3))
  (bind (_projectedlocation _returnvalue_4) (AI|Navigation|ProjectPointtoNavigation _returnvalue 0 0 "200.000000,200.000000,200.000000"))
  (bind (_projectedlocation_2 _returnvalue_5) (AI|Navigation|ProjectPointtoNavigation _returnvalue_2 0 0 "200.000000,200.000000,200.000000"))
  (bind (_projectedlocation_3 _returnvalue_6) (AI|Navigation|ProjectPointtoNavigation _returnvalue_3 0 0 "200.000000,200.000000,200.000000"))
  ;[1 1 1] Spawn targets according to type, and event rate
  (if (>= (- (Variables|Default|GetArraySize) (Variables|Default|GetSpawnIndex)) 0)
    (switch Utilities|FlowControl|Switch|SwitchonTargetCycleEnum (Utilities|Array|Get(acopy) (Variables|Default|GetCycleArray) (Variables|Default|GetSpawnIndex))
      (:NewEnumerator4
        (if _returnvalue_5
          (bind _returnvalue_7 (AI|SpawnAIFromClass "/Game/Blueprints/AI/HumanoidAI_Exo/HTarget1.HTarget1_C" 0 _projectedlocation_2 (Transformation|GetWorldRotation _spawn_2) false))
          (CallFunction|AssignDestinationfromID _returnvalue_7)
          (else
            (Development|PrintString "projectionfailed"))))
      (:NewEnumerator5
        (if _returnvalue_6
          (bind _returnvalue_8 (AI|SpawnAIFromClass "/Game/Blueprints/AI/HumanoidAI_Swat/HNoise1.HNoise1_C" 0 _projectedlocation_3 (Transformation|GetWorldRotation _spawn_3) false))
          (CallFunction|AssignDestinationfromID _returnvalue_8)
          (else
            (Development|PrintString "projectionfailed"))))
      (:NewEnumerator6
        (if _returnvalue_4
          (bind _returnvalue_9 (AI|SpawnAIFromClass "/Game/Blueprints/AI/HumanoidAI_Swat/HNoise2.HNoise2_C" 0 _projectedlocation (Transformation|GetWorldRotation _spawn) false))
          (CallFunction|AssignDestinationfromID _returnvalue_9)
          (else
            (Development|PrintString "projectionfailed")))))
    (else
      (Variables|Default|SetSpawnIndex 0))))

(fn AssignDestinationfromID
  (params (TargetToCommand :type Actor%20Object%20Reference))
  (switch Utilities|FlowControl|Switch|SwitchonSpawnerNumber (Variables|Default|GetSpawnerID)
    (:NewEnumerator4
      (Class|SpawnInterface|AssignDestination(Message) TargetToCommand (Utilities|Array|Get(acopy) (Variables|Default|GetHDestinationArray1) (Variables|Default|GetSpawnIndex)))
      (Variables|Default|SetSpawnIndex (+ (Variables|Default|GetSpawnIndex) 1)))))