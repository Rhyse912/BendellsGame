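; VR magazine actor that loads itself into a compatible realistic gun when its collision overlaps it.
; Compatibility matches its class, or a parent class, against the gun's list, then the hand's physics handle releases it.
; Collision and physics switch off, and a timeline slides the mesh to the gun root before attaching it to the frame.
; Construction optionally fills ammo from the first entry, and dropping re-enables magazine collision after a delay.
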(event OnComponentBeginOverlap(MagazineCollision)
  (params (OverlappedComponent :type Primitive%20Component%20Object%20Reference) (OtherActor :type Actor%20Object%20Reference) (OtherComp :type Primitive%20Component%20Object%20Reference) (OtherBodyIndex :type Integer) (bFromSweep :type Boolean) (SweepResult :type Hit%20Result%20Structure%20%28by%20ref%29))
  ;[0.03215 1 0.8703] Animate Magazine and attach it to Gun
  (bind _asbp_vrrealistic_gun_base (Utilities|Casting|CastToBP_VRRealisticGun_Base OtherActor)
    (:then
      (bind _returnvalue (|CheckIfCompatible _asbp_vrrealistic_gun_base))
      (if _returnvalue
        (CallFunction|ReleaseThisMagazinefromHand)
        (|AnimateMagazineEjectionandsetupcollision _asbp_vrrealistic_gun_base)))
    (:CastFailed
      (Development|PrintString "Failed cast to the Gun On Magazine BeginOverlap" false))))

(event Custom|MagazineDropped
  ;[0 0.3185 1] WhenMagDropped, reactivate colision
  (Utilities|FlowControl|Delay 1.0)
  (Collision|SetCollisionEnabled (Variables|Default|GetMagazineCollision) "QueryAndPhysics"))

(fn ConstructionScript
  (bind _ammo (Variables|Default|GetAmmo))
  (bind _item (Utilities|Array|Get(acopy) _ammo))
  ;[1 1 1] Fill Ammo
  (if (and (Utilities|IsValidClass _item) (Variables|Default|GetFillMagazine))
    (for _index (range 1 (- (Variables|Default|GetMaxAmmo) 1))
      (Utilities|Array|SetArrayElem (Variables|Default|GetAmmo) _index _item true))
    (Variables|Default|SetFillMagazine false)))

(fn ReleaseThisMagazinefromHand
  (bind _outactors (Actor|GetAllActorsOfClass "/Game/VRGunToolkit/Blueprints/Character/BP_VRrGunHands.BP_VRrGunHands_C"))
  (for _array_element _outactors
    (if (== (Variables|/Game/VRGunToolkit/Blueprints/Character/BP_VRrGunHands.BP_VRrGunHands_C|GetGrabbingObject _array_element) (Variables|Default|GetMagazineMesh))
      (Physics|Components|PhysicsHandle|ReleaseComponent (Variables|/Game/VRGunToolkit/Blueprints/Character/BP_VRrGunHands.BP_VRrGunHands_C|GetPhysicsHandle _array_element))
      (Variables|/Game/VRGunToolkit/Blueprints/Character/BP_VRrGunHands.BP_VRrGunHands_C|SetGrabbingObject _array_element 0))))

(fn CheckifClassIsParent
  (params (GroupActor :type Array%20of%20Actor%20Class%20References) (Child :type Object%20Class%20Reference))
  ;[1 1 1] We check if any of the actors are children of the parent
  (bind _array_element (Utilities|Array|ForEachLoopwithBreak GroupActor :!label _label)
    (:LoopBody
      (if (Utilities|ClassIsChildOf Child _array_element)
        (Utilities|FlowControl|Sequence
          (:then_0
            (goto _label Break))
          (:then_1
            (return true)))))
    (:Completed
      (return false))))