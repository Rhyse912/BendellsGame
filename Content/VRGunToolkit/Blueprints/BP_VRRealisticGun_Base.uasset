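; Base Blueprint for a VR gun, simulating trigger, hammer, hand-pulled charging slide, chambered rounds and detachable magazine.
; Racking the slide ejects the chamber and loads from the magazine's ammo array.
; Firing spawns the chambered round as a projectile with effects and haptics, then handles semi-auto cycling, full-auto looping and empty slide lock.
; Slide and magazine-ejection animations use gated Tick-driven lerps instead of timelines, allowing per-gun speeds.
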(event Custom|Fire
  (bind _slidestuck (Variables|Private|GetSlideStuck))
  (bind _returnvalue (not _slidestuck))
  ;[0.7021 1 0.7342] FireLogic
  (if (and (Variables|Private|GetCocked) _returnvalue)
    (if (Variables|GunSettings|GetFullAuto?) :!label _label
      ;;[1 0.3366 0.07409] Automatic/Full Auto Fire Logic
      (Utilities|FlowControl|Sequence
        (:then_0
          (goto _label_2 Open))
        (:then_1
          (Utilities|FlowControl|Gate true :!label _label_2
            (:Exit
              _)))))
    (Variables|Private|SetCocked false)
    (if (!= (Variables|Private|GetChamber) "/Game/VRGunToolkit/Blueprints/Projectiles/Private/BP_EmptyRound_DoNotEdit.BP_EmptyRound_DoNotEdit_C")
      ;;[1 0.0148 0] Fire Logic
      (|FireLogic :!label _label_3)
      (else
        ;;[1 0.7535 0.3812] Check if this Gun gets ammo directly from the magazine
        (if (Variables|GunSettings|GetGetsAmmoDirectlyFromMagazine)
          (bind _successful (CallFunction|GetAmmofromMagazine))
          (if _successful
            (goto _label_3)
            (else
              _)))
        ;;[1 0.7778 0.5373] Out of ammo
        (Audio|PlaySound2D (Variables|Sound&Effects|GetOutOfAmmoSound) 1.0 1.0)
        (Transformation|SetRelativeRotation (Variables|Default|GetHammerRotationOffset) (Variables|Private|GetInitialHammerRotation) false false)))
    (elif (and (Variables|GunSettings|GetDoubleAction) _returnvalue)
      (goto _label))))

(event Custom|UnlockSlider
  ;[1 0.9829 0.6764] Unlock Slider
  (if (Variables|Private|GetSlideStuck)
    (Transformation|SetRelativeLocation (Variables|Default|GetSlider) (Variables|Private|GetSlideInitialPosition) false false)
    (CallFunction|SlideForward)))

(event Custom|FireLoop
  ;[0.7021 1 0.7342] FireLogic
  ;;[1 0.3366 0.07409] Automatic/Full Auto Fire Logic
  (Utilities|FlowControl|Delay (Variables|GunSettings|GetFullAutoDelay))
  (Utilities|FlowControl|Gate true
    (:Exit
      (Variables|Private|SetCocked false)
      (if (!= (Variables|Private|GetChamber) "/Game/VRGunToolkit/Blueprints/Projectiles/Private/BP_EmptyRound_DoNotEdit.BP_EmptyRound_DoNotEdit_C")
        ;;[1 0.0148 0] Fire Logic
        (|FireLogic :!label _label)
        (else
          ;;[1 0.7535 0.3812] Check if this Gun gets ammo directly from the magazine
          (if (Variables|GunSettings|GetGetsAmmoDirectlyFromMagazine)
            (bind _successful (CallFunction|GetAmmofromMagazine))
            (if _successful
              (goto _label)
              (else
                _)))
          ;;[1 0.7778 0.5373] Out of ammo
          (Audio|PlaySound2D (Variables|Sound&Effects|GetOutOfAmmoSound) 1.0 1.0)
          (Transformation|SetRelativeRotation (Variables|Default|GetHammerRotationOffset) (Variables|Private|GetInitialHammerRotation) false false))))))

(event Custom|SlideMoveAction
  (params (Locationoffset :type Vector) (HandGrabbingSlider :type Motion%20Controller%20Component%20Object%20Reference))
  (bind _returnvalue (Transformation|GetWorldLocation HandGrabbingSlider))
  (bind _self self)
  (bind _self_2 self)
  (bind (_returnvalue_2 _returnvalue2) (Utilities|DetermineSliderHandPosition Locationoffset _returnvalue _self_2))
  ;[0.7362 0.6537 1] Slider/Charging
  (Transformation|SetRelativeLocation (Variables|BP_VRRealisticGun_Base_C|GetChargingMechanism self) _returnvalue2 false false)
  (if (and (not (Variables|Private|GetSlideStuck)) (Math|Vector|Equal(Vector) (Variables|/Script/Engine.SceneComponent|GetRelativeLocation (Variables|BP_VRRealisticGun_Base_C|GetChargingMechanism _self)) (Variables|BP_VRRealisticGun_Base_C|GetChargingMechanismEndPoint _self) 0.1))
    (CallFunction|SlideBack)
    (goto _label Reset)
    (elif (and (Variables|BP_VRRealisticGun_Base_C|GetCocked _self_2) _returnvalue_2)
      (Utilities|FlowControl|DoOnce false :!label _label
        (:Completed
          (CallFunction|SlideForward))))))

(event Custom|ReleaseMagazine
  ;[0.4605 0.91 1] DropMagazine
  (if (and (Utilities|IsValid (Variables|MagazineSetup|GetMagazine)) (Variables|GunSettings|GetAllowMagazineRelease/Ejection))
    (Audio|PlaySoundatLocation (Variables|Sound&Effects|GetMagazineDropSound) (Transformation|GetActorLocation))
    (|AnimateMagEjection
      (:AnimationFinished
        (Transformation|DetachFromActor (Variables|MagazineSetup|GetMagazine) "KeepWorld" "KeepWorld" "KeepWorld")
        (Collision|SetCollisionEnabled (Variables|/Game/VRGunToolkit/Blueprints/BP_VRRealisticMagazine.BP_VRRealisticMagazine_C|GetMagazineMesh (Variables|MagazineSetup|GetMagazine)) "QueryAndPhysics")
        (Physics|SetSimulatePhysics (Variables|/Game/VRGunToolkit/Blueprints/BP_VRRealisticMagazine.BP_VRRealisticMagazine_C|GetMagazineMesh (Variables|MagazineSetup|GetMagazine)) true)
        (Physics|AddForce (Variables|/Game/VRGunToolkit/Blueprints/BP_VRRealisticMagazine.BP_VRRealisticMagazine_C|GetMagazineMesh (Variables|MagazineSetup|GetMagazine)) (* (Math|Vector|RotateVector (Math|Vector|Normalize (Variables|/Script/Engine.SceneComponent|GetRelativeLocation (Variables|Default|GetMagazineEjectionTarget))) (Transformation|GetActorRotation)) (Variables|MagazineSetup|GetMagEjectionForce)) "None" true)
        (Default|MagazineDropped (Variables|MagazineSetup|GetMagazine))
        (Variables|MagazineSetup|SetMagazine 0)
        (Collision|SetCollisionEnabled (Variables|Default|GetMagazineTrigger) "QueryAndPhysics") ; Allow for new magazine to be inserted
      ))))

(event Custom|StopFire
  ;[0.7021 1 0.7342] FireLogic
  ;;[1 0.3366 0.07409] Automatic/Full Auto Fire Logic
  (Utilities|FlowControl|Gate true) ; enters at Close
)

(event Custom|SlideSprintForward
  ;[0.7362 0.6537 1] Slider/Charging
  (Utilities|FlowControl|DoOnce false
    (:Completed
      (CallFunction|SlideForward))))

(event EventBeginPlay
  ;[0.2904 0.4084 0.465] BeginPlay
  (Variables|Private|SetInitialTriggerRotation (Variables|/Script/Engine.SceneComponent|GetRelativeRotation (Variables|Default|GetTriggerRotationOffset)))
  (Variables|Private|SetSlideInitialPosition (Variables|/Script/Engine.SceneComponent|GetRelativeLocation (Variables|Default|GetChargingMechanism)))
  (Variables|Private|SetInitialHammerRotation (Variables|/Script/Engine.SceneComponent|GetRelativeRotation (Variables|Default|GetHammerRotationOffset))))

(event EventTick
  (params (DeltaSeconds :type Float%20%28single-precision%29))
  ;[0.13 0.0407 0.1141] Tick
  (Utilities|FlowControl|Sequence
    (:then_0
      ;;[1 1 1] TriggerAnim
      (Transformation|SetRelativeRotation (Variables|Default|GetTriggerRotationOffset) (Math|Rotator|Lerp(Rotator) (Variables|Private|GetInitialTriggerRotation) (Variables|GunSettings|GetTriggerRotationEndPoint) (Variables|Private|GetTriggerAxis)) false false))
    (:then_1
      ;;[0 0.9923 1] Slider Firing Animation Tick
      (CallFunction|SliderFiringTick DeltaSeconds))
    (:then_2
      ;;[0 0.5892 1] Mag ejection Animation Tick
      (CallFunction|MagEjectionTick DeltaSeconds))))

(fn ConstructionScript
  (bind _hammer (Variables|Default|GetHammer))
  (bind _trigger (Variables|Default|GetTrigger))
  (bind _triggerrotationoffset (Variables|Default|GetTriggerRotationOffset))
  (bind _hammerrotationoffset (Variables|Default|GetHammerRotationOffset))
  (Transformation|SetRelativeTransform _hammer (Math|Transform|MakeTransform (* (Variables|/Script/Engine.SceneComponent|GetRelativeLocation _hammerrotationoffset) -1.0) (Variables|/Script/Engine.SceneComponent|GetRelativeRotation _hammer) (Variables|/Script/Engine.SceneComponent|GetRelativeScale3D _hammerrotationoffset)) false false)
  (Transformation|SetRelativeTransform _trigger (Math|Transform|MakeTransform (* (Variables|/Script/Engine.SceneComponent|GetRelativeLocation _triggerrotationoffset) -1.0) (Variables|/Script/Engine.SceneComponent|GetRelativeRotation _trigger) (Variables|/Script/Engine.SceneComponent|GetRelativeScale3D _triggerrotationoffset)) false false)
  (if (not (Variables|GunSettings|GetAllows2HandGrip))
    (Components|DestroyComponent (Variables|Default|Get2ndHandGrab))))

(fn GetAmmofromMagazine
  (bind _magazine (Variables|MagazineSetup|GetMagazine))
  (bind _ammo (Variables|/Game/VRGunToolkit/Blueprints/BP_VRRealisticMagazine.BP_VRRealisticMagazine_C|GetAmmo _magazine))
  (Utilities|IsValid (Variables|MagazineSetup|GetMagazine)
    (:Is%20Valid
      (if (> (Utilities|Array|Length _ammo) 0)
        (Variables|Private|SetChamber (Utilities|Array|Get(acopy) _ammo))
        (Utilities|Array|RemoveIndex _ammo)
        (return true)
        (else
          _)))
    (:Is%20Not%20Valid
      _))
  (return false))

(fn SlideBack
  (Variables|Private|SetCocked true)
  (Variables|Private|SetSlideStuck true)
  (Transformation|SetRelativeRotation (Variables|Default|GetHammerRotationOffset) (Variables|GunSettings|GetHammerRotationEndPoint) false false)
  (Audio|PlaySound2D (Variables|Sound&Effects|GetSliderBackSound))
  (if (!= (Variables|Private|GetChamber) "/Game/VRGunToolkit/Blueprints/Projectiles/Private/BP_EmptyRound_DoNotEdit.BP_EmptyRound_DoNotEdit_C")
    (CallFunction|ShellEject (Variables|Private|GetChamberRoundShot))
    (Variables|Private|SetChamber "/Game/VRGunToolkit/Blueprints/Projectiles/Private/BP_EmptyRound_DoNotEdit.BP_EmptyRound_DoNotEdit_C")))

(fn SlideForward
  (bind _self self)
  (Variables|BP_VRRealisticGun_Base_C|SetCocked _self true)
  (Variables|BP_VRRealisticGun_Base_C|SetSlideStuck _self false)
  (Audio|PlaySound2D (Variables|Sound&Effects|GetSliderForwardSound))
  (CallFunction|GetAmmofromMagazine _self)
  (Transformation|SetRelativeRotation (Variables|BP_VRRealisticGun_Base_C|GetHammerRotationOffset _self) (Variables|BP_VRRealisticGun_Base_C|GetHammerRotationEndPoint _self) false false)
  (Variables|Private|SetChamberRoundShot false))

(fn ShellEject
  (params (Fired :type Boolean))
  (bind _ejectionpositionandrotation (Variables|Default|GetEjectionPositionAndRotation))
  (bind _returnvalue (Transformation|GetWorldTransform _ejectionpositionandrotation))
  (bind _returnvalue_2 (Game|SpawnActorfromClass (Variables|Private|GetChamber) (Math|Transform|MakeTransform (.location _returnvalue) (.rotation _returnvalue) "1,1,1") "Undefined" 0 0))
  (Default|ShellOnly _returnvalue_2 Fired)
  (Physics|SetPhysicsLinearVelocity (Variables|/Game/VRGunToolkit/Blueprints/BP_Ammo_Projectile_Base.BP_Ammo_Projectile_Base_C|GetShell _returnvalue_2) (* (Math|Vector|GetForwardVector (Variables|Default|GetEjectionPositionAndRotation)) (Variables|GunSettings|GetShellEjectionForce)) false "None"))

(event Custom|MagEjectionTick
  (params (A :type Float%20%28single-precision%29))
  ;[1 1 1] Instead of doing a fixed timed timeline, we use a variable that we can edit for each gun, increasing/decreasing the amount of time the slider takes to move. We take the tick delta and add it to a Var until it reached >1
  (Utilities|FlowControl|Gate true :!label _label
    (:Exit
      (Transformation|SetRelativeLocation (Variables|/Game/VRGunToolkit/Blueprints/BP_VRRealisticMagazine.BP_VRRealisticMagazine_C|GetMagazineMesh (Variables|MagazineSetup|GetMagazine)) (Math|Vector|Lerp(Vector) "0, 0, 0" (Variables|/Script/Engine.SceneComponent|GetRelativeLocation (Variables|Default|GetMagazineEjectionTarget)) (Variables|Private|GetMagazineAnimAlpha)) false false)
      (bind _output_get (Variables|Private|SetMagazineAnimAlpha (+ (/ A (Variables|MagazineSetup|GetMagEjecTime)) (Variables|Private|GetMagazineAnimAlpha))))
      (if (>= _output_get 1.0)
        (Utilities|FlowControl|DoOnce false :!label _label_2
          (:Completed
            (Utilities|FlowControl|Sequence
              (:then_0
                (return))
              (:then_1
                (goto _label Close))
              (:then_2
                (goto _label_2 Reset))
              (:then_3
                (Variables|Private|SetMagazineAnimAlpha 0.0)))))))))

(event Custom|StopSliderTick
  (Utilities|FlowControl|Gate true) ; enters at Close
)

(event Custom|SliderFiringTick
  (params (NewParam :type Float%20%28single-precision%29))
  (Utilities|FlowControl|Gate true
    (:Exit
      ;[1 1 1] Animate with variable speed
      (Transformation|SetRelativeLocation (Variables|Default|GetSlider) (select (>= (Variables|Private|GetSliderAnimAlpha) 1.0) (Math|Vector|Lerp(Vector) (Variables|GunSettings|GetChargingMechanismEndPoint) (Variables|Private|GetSlideInitialPosition) (- (Variables|Private|GetSliderAnimAlpha) 1.0)) (Math|Vector|Lerp(Vector) (Variables|Private|GetSlideInitialPosition) (Variables|GunSettings|GetChargingMechanismEndPoint) (Variables|Private|GetSliderAnimAlpha))) false false)
      (bind _output_get (Variables|Private|SetSliderAnimAlpha (+ (* NewParam (Variables|GunSettings|GetSliderFiringMovementSpeed)) (Variables|Private|GetSliderAnimAlpha))))
      (if (>= _output_get 1.0)
        ;[0.5212 1 0.6338] IfEmptySlideLock
        (if (and (== (Variables|Private|GetChamber) "/Game/VRGunToolkit/Blueprints/Projectiles/Private/BP_EmptyRound_DoNotEdit.BP_EmptyRound_DoNotEdit_C") (Variables|GunSettings|GetSlideLocks?))
          (Transformation|SetRelativeLocation (Variables|Default|GetSlider) (- (Variables|GunSettings|GetChargingMechanismEndPoint) (Variables|Private|GetSlideInitialPosition)) false false)
          (Variables|Private|SetSlideStuck true)
          (CallFunction|StopSliderTick)
          (else
            ;[1 1 1] If Slide does not lock, then move forward back to original position
            (if (>= (Variables|Private|GetSliderAnimAlpha) 2.0)
              (Transformation|SetRelativeLocation (Variables|Default|GetSlider) (Variables|Private|GetSlideInitialPosition) false false)
              (CallFunction|StopSliderTick))))))))