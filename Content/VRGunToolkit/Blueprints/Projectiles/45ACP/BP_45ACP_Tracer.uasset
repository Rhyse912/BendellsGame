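; BP_45ACP_Tracer is a .45 ACP tracer projectile that draws an orange trail behind the bullet.
; It records its spawn location on BeginPlay, and its BulletOnly event runs the parent logic, then opens a gate.
; While the gate is open, each Tick draws a short-lived debug line from the last location to the current one, using debug drawing as the tracer visual.
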(event EventBeginPlay
  ;[0.1963 0.362 1] BeginPlay we take the spawn location as the start of the debug Draw
  (Variables|Default|SetLastLocation (Transformation|GetActorLocation)))

(event EventTick
  (params (DeltaSeconds :type Float%20%28single-precision%29))
  (bind _returnvalue (Transformation|GetActorLocation))
  ;[0 1 0.3223] Draw debug line behind the bullet
  (Utilities|FlowControl|Gate true
    (:Exit
      (Rendering|Debug|DrawDebugLine (Variables|Default|GetLastLocation) _returnvalue "(R=1.000000,G=0.092126,B=0.000000,A=1.000000)" 1.0 1.5)
      (Variables|Default|SetLastLocation _returnvalue))))

(event EventBulletOnly
  (bind _returnvalue (Transformation|GetActorLocation))
  ;[0 1 0.3223] Draw debug line behind the bullet
  (|CallParentFunction)
  (Utilities|FlowControl|Gate true) ; enters at Open
)

(fn ConstructionScript
  (|CallParentFunction))